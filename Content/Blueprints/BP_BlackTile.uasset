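; BP_BlackTile is a clickable board tile, apparently the black square of a board game with pieces.
; Clicking its static mesh casts itself to Tile and passes it to the board reference's TileClicked, leaving the response to the board.
; It then prints the tile's X and Y coordinates and has its piece print its type, with no validity check on that piece.
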(event `self.StaticMeshComponent.OnClicked`
  (params (TouchedComponent :type "PrimitiveComponent Object Reference") (ButtonPressed :type "Key Structure"))
  (bind _astile (cast `Tile` self))
  (bind _returnvalue (`self.GetTileInfo`))
  (`Board.TileClicked` (`self.BoardRef`) _astile)
  (bind (_x _y) (break `TileInfo` _returnvalue))
  (`KismetSystemLibrary.PrintString` (`KismetStringLibrary.Concat_StrStr` (`KismetStringLibrary.Conv_IntToString` _x) (`KismetStringLibrary.Conv_IntToString` _y)))
  (bind _returnvalue_2 (`self.GetPiece`))
  (`ChessPiece.PrintType` _returnvalue_2))

(fn `UserConstructionScript`)